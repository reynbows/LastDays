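; Game instance Blueprint for LAN multiplayer, handling requests to host or join a lobby.
; Hosting creates a LAN session, then opens the Showcase map as a listen server through a console command.
; Joining skips session search and runs an open console command built from the supplied IP.
; Session find-and-join and alternative level-opening paths remain in the graph but are disconnected.
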(event `GameInstance_HostLobby`
  (params (Host :type "/Game/Blueprints/BP_PlayerController Object Reference"))
  (`CreateSessionCallbackProxy.CreateSession` Host 100 true
    (:`OnSuccess`
      (`KismetSystemLibrary.ExecuteConsoleCommand` "open Showcase?Listen" Host)
      (`KismetSystemLibrary.PrintString` "Open suceeded"))
    (:`OnFailure`
      (`KismetSystemLibrary.PrintString` "Session Create Failed" true true (struct :`R` 1.0 :`G` 0.030483 :`A` 1.0)))))

(event `GameInstance_JoinLobby`
  (params (Joining :type "/Game/Blueprints/BP_PlayerController Object Reference") (IP :type String))
  (bind _returnvalue (`KismetStringLibrary.Concat_StrStr` (`KismetTextLibrary.Conv_TextToString` (`|FormatText` "open ")) IP))
  (`KismetSystemLibrary.ExecuteConsoleCommand` _returnvalue Joining)
  (`KismetSystemLibrary.PrintString` _returnvalue))