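; Multiplayer player controller that toggles a lobby menu with Tab and switches possession between third-person characters and four camera-plane pawns.
; Host and join events forward to BP_MPGameInstance.
; Modifier-plus-number keys send camera transform and modifier state through RPC_PossessPawn: 0 takes an uncontrolled character.
; For 1–4, Shift possesses that plane, Ctrl also moves its camera to the current view, and Cmd alone rotates it toward the controlled character.
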(event `self.ReceiveBeginPlay`
  ;[1 1 1] Creating the Startup Menu
  (`KismetSystemLibrary.Delay` 2.0)
  (`/Engine/EditorBlueprintResources/ActorMacros.Switch Has Authority`
    (:`Authority`
      (`self.Player_CreateMenu`))))

(event `Player_CreateMenu`
  ;[1 1 1] Creating the Startup Menu
  (bind _returnvalue (`|CreateWidget` "/Game/Blueprints/BP_Menu.BP_Menu_C" self))
  (bind _output_get (set `self.Player_Menu` _returnvalue))
  (`UserWidget.AddToViewport` _output_get 0)
  (`Widget.SetVisibility` _output_get "Hidden"))

(event `Key|Tab`
  (params (Key :type "Key Structure"))
  (bind _player_menu (`self.Player_Menu`))
  ;[1 1 1] Creating the Startup Menu
  (:`Pressed`
    (if (`|EnumEquality` (`Widget.GetVisibility` (`self.Player_Menu`)) "Visible")
      (`Widget.SetVisibility` _player_menu "Hidden")
      (`WidgetBlueprintLibrary.SetInputMode_GameOnly` self)
      (set `self.bShowMouseCursor` false)
      (else
        (`Widget.SetVisibility` _player_menu "Visible")
        (`WidgetBlueprintLibrary.SetInputMode_GameAndUIEx` self (`self.Player_Menu`))
        (set `self.bShowMouseCursor` true)))))

(event `Player_Server_HostLobby`
  ;[1 1 1] Hosting/Joining Game
  (bind _asbp_mpgame_instance (cast `/Game/Blueprints/GhMP/Blueprints/BP_MPGameInstance` (`GameplayStatics.GetGameInstance`))
    (:`then`
      (`/Game/Blueprints/GhMP/Blueprints/BP_MPGameInstance.GameInstance_HostLobby` _asbp_mpgame_instance self))
    (:`CastFailed`
      (`KismetSystemLibrary.PrintString` "failed"))))

(event `Player_Server_JoinLobby`
  (params (IP :type String))
  ;[1 1 1] Hosting/Joining Game
  (bind _asbp_mpgame_instance (cast `/Game/Blueprints/GhMP/Blueprints/BP_MPGameInstance` (`GameplayStatics.GetGameInstance`)))
  (`/Game/Blueprints/GhMP/Blueprints/BP_MPGameInstance.GameInstance_JoinLobby` _asbp_mpgame_instance self IP))

(event `Key|LeftShift`
  (params (Key :type "Key Structure"))
  ;[1 1 1] Keyboard Input to Select Possessed Pawn
  (:`Pressed`
    (set `self.ShiftDown` true))
  (:`Released`
    (set `self.ShiftDown` false)))

(event `Key|LeftControl`
  (params (Key :type "Key Structure"))
  ;[1 1 1] Keyboard Input to Select Possessed Pawn
  (:`Pressed`
    (set `self.CtrlDown` true))
  (:`Released`
    (set `self.CtrlDown` false)))

(event `Key|LeftCommand`
  (params (Key :type "Key Structure"))
  ;[1 1 1] Keyboard Input to Select Possessed Pawn
  (:`Pressed`
    (set `self.CmdDown` true))
  (:`Released`
    (set `self.CmdDown` false)))

(event `Key|One`
  (params (Key :type "Key Structure"))
  (bind _returnvalue (`GameplayStatics.GetPlayerCameraManager` 0))
  ;[1 1 1] Keyboard Input to Select Possessed Pawn
  (:`Pressed`
    (set `self.KeyStructPressed` Key)
    (if (or (`self.ShiftDown`) (`self.CtrlDown`) (`self.CmdDown`)) :!label _label
      (`self.RPC_PossessPawn` (`GameplayStatics.GetPlayerController` 0) (`self.KeyStructToInt` (`self.KeyStructPressed`)) (`self.CtrlDown`) (`self.CmdDown`) (`self.ShiftDown`) (`KismetMathLibrary.MakeTransform` (`PlayerCameraManager.GetCameraLocation` _returnvalue) (`PlayerCameraManager.GetCameraRotation` _returnvalue))))))

(event `RPC_PossessPawn`
  (params (thePlayerController :type "PlayerController Object Reference") (PlaneNumber :type Integer) (Ctrl :type Boolean) (Cmd :type Boolean) (Shift :type Boolean) (cameraTransform :type "Transform Structure"))
  (bind _thepawn (`self.thePawn`))
  (bind _thepawn_2 (`self.thePawn`))
  ;[1 1 1] Possess Relevant Pawn and Update Transform
  (set `self.passedPlayerController` thePlayerController)
  (set `self.passedCtrl` Ctrl)
  (set `self.passedCmd` Cmd)
  (set `self.passedShift` Shift)
  (set `self.passedCamTransform` cameraTransform)
  (switch `int` PlaneNumber
    (:`0`
      (bind _outactors (`GameplayStatics.GetAllActorsOfClass` "/Game/ThirdPersonCPP/Blueprints/ThirdPersonCharacter.ThirdPersonCharacter_C"))
      (for _array_element _outactors
        (if (not (`Pawn.IsPlayerControlled` _array_element))
          (`self.Possess` _array_element))))
    (:`1`
      (bind _returnvalue (`GameplayStatics.GetActorOfClass` "/Game/Blueprints/BP_CameraPlane_0.BP_CameraPlane_0_C"))
      (set `self.thePawn` _returnvalue)
      (if (or (`self.passedShift`) (`self.passedCtrl`)) :!label _label_2
        (if (not (`Pawn.IsPlayerControlled` (`self.thePawn`)))
          (if (`self.passedCtrl`)
            (`self.SetCameraOffsetRef`)
            (`SceneComponent.K2_SetWorldTransform` (`self.GetComponentByClass` _thepawn "/Script/Engine.CameraComponent") (`self.CamTransformRef`) false false))
          (`self.Possess` (`self.passedPlayerController`) _thepawn))
        (else
          (bind _outactors_2 (`GameplayStatics.GetAllActorsOfClass` "/Game/ThirdPersonCPP/Blueprints/ThirdPersonCharacter.ThirdPersonCharacter_C"))
          (for _array_element_2 _outactors_2
            (if (== _array_element_2 (`self.K2_GetPawn`))
              (bind _asbp_camera_plane_parent (cast `/Game/Blueprints/BP_CameraPlaneParent` _thepawn_2)
                (:`then`
                  (`/Game/Blueprints/BP_CameraPlaneParent.RotatePlaneToCharacter` _asbp_camera_plane_parent _array_element_2 _thepawn_2))
                (:`CastFailed`
                  (`KismetSystemLibrary.PrintString` "Cast to BPPArent failer"))))))))
    (:`2`
      (bind _returnvalue_2 (`GameplayStatics.GetActorOfClass` "/Game/Blueprints/BP_CameraPlane_1.BP_CameraPlane_1_C"))
      (set `self.thePawn` _returnvalue_2)
      (goto _label_2))
    (:`3`
      (bind _returnvalue_3 (`GameplayStatics.GetActorOfClass` "/Game/Blueprints/BP_CameraPlane_2.BP_CameraPlane_2_C"))
      (set `self.thePawn` _returnvalue_3)
      (goto _label_2))
    (:`4`
      (bind _returnvalue_4 (`GameplayStatics.GetActorOfClass` "/Game/Blueprints/BP_CameraPlane_3.BP_CameraPlane_3_C"))
      (set `self.thePawn` _returnvalue_4)
      (goto _label_2))))

(event `Key|Two`
  (params (Key :type "Key Structure"))
  ;[1 1 1] Keyboard Input to Select Possessed Pawn
  (:`Pressed`
    (set `self.KeyStructPressed` Key)
    (goto _label)))

(event `Key|Three`
  (params (Key :type "Key Structure"))
  ;[1 1 1] Keyboard Input to Select Possessed Pawn
  (:`Pressed`
    (set `self.KeyStructPressed` Key)
    (goto _label)))

(event `Key|Four`
  (params (Key :type "Key Structure"))
  ;[1 1 1] Keyboard Input to Select Possessed Pawn
  (:`Pressed`
    (set `self.KeyStructPressed` Key)
    (goto _label)))

(event `self.ReceiveTick`
  (params (DeltaSeconds :type "Float (single-precision)")))

(event `Key|Zero`
  (params (Key :type "Key Structure"))
  ;[1 1 1] Keyboard Input to Select Possessed Pawn
  (:`Pressed`
    (set `self.KeyStructPressed` Key)
    (goto _label)))

(event `RPC Server Pawn Transform`
  (params (transform :type "Transform Structure"))
  (set `self.pawnTransform` transform))

(fn `OnRep_pawnTransform`
  (`self.K2_SetActorTransform` (`self.pawnTransform`)))

(fn `SetCameraOffsetRef`
  (bind _passedcamtransform (`self.passedCamTransform`))
  (`KismetSystemLibrary.PrintString` (`KismetStringLibrary.Conv_TransformToString` _passedcamtransform))
  (set `self.CamTransformRef` _passedcamtransform)
  (return))

(fn `UserConstructionScript`)