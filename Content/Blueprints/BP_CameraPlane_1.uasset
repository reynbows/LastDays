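; BP_CameraPlane_1 is a camera plane Blueprint that creates a material instance and updates it every frame.
; After a half-second delay on BeginPlay, it calls the parent's BeginPlay, stores the result of InitializeCameraPlane as its material instance and sets Pause true.
; Tick passes that instance to GlobalTick only while Pause is true, so the flag acts as a ready gate despite its name.
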(event `self.ReceiveBeginPlay`
  (`KismetSystemLibrary.Delay` 0.5)
  (`parent.ReceiveBeginPlay`)
  (bind _thematerialinstance (`self.InitializeCameraPlane`))
  (set `self.myMaterialInstance` _thematerialinstance)
  (set `self.Pause` true))

(event `self.ReceiveTick`
  (params (DeltaSeconds :type "Float (single-precision)"))
  (`parent.ReceiveTick` DeltaSeconds)
  (if (`self.Pause`)
    (`self.GlobalTick` (`self.myMaterialInstance`))))

(fn `UserConstructionScript`
  (`parent.UserConstructionScript`))